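; Coin pickup actor for a side-scroller that adds to the player's coin tally and score when collected.
; A Box overlap by SideScrollerCharacter, or any hit on the Box, plays a coin sound, passes its values to the Instancia_Anahuac GameInstance, then destroys the actor.
; Each event has its own DoOnce guard, and only the overlap path checks the other actor's class.
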(event OnComponentBeginOverlap(Box)
  (params (OverlappedComponent :type Primitive%20Component%20Object%20Reference) (OtherActor :type Actor%20Object%20Reference) (OtherComp :type Primitive%20Component%20Object%20Reference) (OtherBodyIndex :type Integer) (bFromSweep :type Boolean) (SweepResult :type Hit%20Result%20Structure%20%28by%20ref%29))
  (Utilities|Casting|CastToSideScrollerCharacter OtherActor)
  (Utilities|FlowControl|DoOnce false
    (:Completed
      (Audio|PlaySound2D "/Game/Sound/242857__plasterbrain__coin-get.242857__plasterbrain__coin-get" 1.0 1.0 0.0 0 0)
      (bind _asinstancia_anahuac (Utilities|Casting|CastToInstancia_Anahuac (Game|GetGameInstance)))
      (Default|PuntajeFinalDeMoneda _asinstancia_anahuac (Variables|Default|GetValor_2))
      (Default|AgregarMonedas _asinstancia_anahuac (Variables|Default|GetValor))
      (Actor|DestroyActor))))

(event OnComponentHit(Box)
  (params (HitComponent :type Primitive%20Component%20Object%20Reference) (OtherActor :type Actor%20Object%20Reference) (OtherComp :type Primitive%20Component%20Object%20Reference) (NormalImpulse :type Vector :default "0, 0, 0") (Hit :type Hit%20Result%20Structure%20%28by%20ref%29))
  (Utilities|FlowControl|DoOnce false
    (:Completed
      (Audio|PlaySound2D "/Game/Sound/242857__plasterbrain__coin-get.242857__plasterbrain__coin-get" 1.0 1.0 0.0 0 0)
      (bind _asinstancia_anahuac (Utilities|Casting|CastToInstancia_Anahuac (Game|GetGameInstance)))
      (Default|PuntajeFinalDeMoneda _asinstancia_anahuac (Variables|Default|GetValor_2))
      (Default|AgregarMonedas _asinstancia_anahuac (Variables|Default|GetValor))
      (Actor|DestroyActor))))

(event EventBeginPlay)

(event Collision|EventActorBeginOverlap
  (params (OtherActor :type Actor%20Object%20Reference)))

(event EventTick
  (params (DeltaSeconds :type Float%20%28single-precision%29)))

(fn ConstructionScript)