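; Bridge Blueprint built from many static mesh pieces that can collapse under physics.
; The ActivaGravedad custom event turns on physics simulation for the listed mesh components in one call, leaving StaticMesh23 out.
; Nothing in this Blueprint calls the event, and the construction script is empty.
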(event Custom|ActivaGravedad
  (Physics|SetSimulatePhysics (Variables|Default|GetStaticMesh) true))

(fn ConstructionScript)