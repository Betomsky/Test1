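; End-of-level flagpole for level 3 of a Mario-style side-scroller.
; Touching the pole once disables input, destroys the Reloj clock, signals the music to stop, plays sounds, lowers the flag and drops pole collision.
; Tick then auto-walks the player onward.
; If the top zone was already reached, fireworks fire and Nivel4 loads after a delay; otherwise the main menu loads.
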(event OnComponentBeginOverlap(ZonadePoste)
  (params (OverlappedComponent :type Primitive%20Component%20Object%20Reference) (OtherActor :type Actor%20Object%20Reference) (OtherComp :type Primitive%20Component%20Object%20Reference) (OtherBodyIndex :type Integer) (bFromSweep :type Boolean) (SweepResult :type Hit%20Result%20Structure%20%28by%20ref%29))
  (bind _asside_scroller_character (Utilities|Casting|CastToSideScrollerCharacter OtherActor))
  (Utilities|FlowControl|DoOnce false
    (:Completed
      (Input|DisableInput _asside_scroller_character (Game|GetPlayerController 0))
      (bind _returnvalue (Actor|GetActorOfClass "/Game/Blueprint/Reloj.Reloj_C"))
      (Actor|DestroyActor _returnvalue)
      (Audio|PlaySound2D "/Game/Sonidos/_Super_Mario_Bros__Mario_Down_the_FlagPole_Sound_Effect__Free_Ringtone_Download_._Super_Mario_Bros__Mario_Down_the_FlagPole_Sound_Effect__Free_Ringtone_Download_" 1.0 1.0 0.0 0 0)
      (Default|CallDetenLaMusica)
      (Components|MoveComponentTo (Variables|Default|GetBandera) "0, 0,-310.000000" "0, 0, 0" true true 1.5 false)
      (Audio|PlaySound2D "/Game/Sonidos/Level_Clear__Classic__-_New_Super_Mario_Bros___OST_.Level_Clear__Classic__-_New_Super_Mario_Bros___OST_" 1.0 1.0 0.0 0 0)
      (Collision|SetCollisionEnabled (Variables|Default|GetPoste) "NoCollision")
      (Variables|Default|SetMueve%20Mario true)
      (if (Variables|Default|GetLlegada%20al%20tope?)
        (Utilities|FlowControl|Sequence
          (:then_0
            (Utilities|FlowControl|Delay 7.0)
            (Game|OpenLevel(byObjectReference) "/Game/Niveles/Nivel4.Nivel4"))
          (:then_1
            (Utilities|FlowControl|Delay 3.0)
            (bind _returnvalue_2 (Actor|GetActorOfClass "/Game/Blueprint/Fuegos_Artificiales.Fuegos_Artificiales_C"))
            (Default|ActivarFuegos _returnvalue_2)))
        (else
          (Utilities|FlowControl|Delay 1e+01)
          (Game|OpenLevel(byObjectReference) "/Game/Niveles/MenuPrincipal.MenuPrincipal"))))))

(event OnComponentBeginOverlap(ZonadeArriba)
  (params (OverlappedComponent :type Primitive%20Component%20Object%20Reference) (OtherActor :type Actor%20Object%20Reference) (OtherComp :type Primitive%20Component%20Object%20Reference) (OtherBodyIndex :type Integer) (bFromSweep :type Boolean) (SweepResult :type Hit%20Result%20Structure%20%28by%20ref%29))
  (Utilities|Casting|CastToSideScrollerCharacter OtherActor)
  (Variables|Default|SetLlegada%20al%20tope? true))

(event EventTick
  (params (DeltaSeconds :type Float%20%28single-precision%29))
  (if (Variables|Default|GetMueve%20Mario)
    (Pawn|Input|AddMovementInput (stale OnComponentBeginOverlap(ZonadePoste) _asside_scroller_character) "0,-1.000000, 0" 1.0 false)))

(fn ConstructionScript)