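; A Mario-style question block for a side-scroller that awards a coin when the player character overlaps its Box trigger.
; The overlap plays a coin sound and, unless QuieresMonedas is set, adds one coin through the Instancia_Anahuac game instance.
; It then fires Brincar to animate the block bump and coin pop with MoveComponentTo, destroys the trigger and swaps in the empty-block mesh.
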(event OnComponentBeginOverlap(Box)
  (params (OverlappedComponent :type Primitive%20Component%20Object%20Reference) (OtherActor :type Actor%20Object%20Reference) (OtherComp :type Primitive%20Component%20Object%20Reference) (OtherBodyIndex :type Integer) (bFromSweep :type Boolean) (SweepResult :type Hit%20Result%20Structure%20%28by%20ref%29))
  (bind _questionblock (Variables|Default|GetQuestionBlock))
  (Utilities|Casting|CastToSideScrollerCharacter OtherActor)
  (Audio|PlaySound2D "/Game/Sound/242857__plasterbrain__coin-get.242857__plasterbrain__coin-get" 1.0 1.0 0.0 0 0)
  (if (not (Variables|Default|GetQuieres%20monedas))
    (bind _asinstancia_anahuac (Utilities|Casting|CastToInstancia_Anahuac (Game|GetGameInstance)))
    (Default|AgregarMonedas _asinstancia_anahuac 1)
    (Utilities|FlowControl|Sequence
      (:then_0
        (CallFunction|Brincar)
        (Components|DestroyComponent (Variables|Default|GetBox))
        (Components|StaticMesh|SetStaticMesh _questionblock "/Game/Geometry/Meshes/EmptyBlock_BlockEmpty__BlockEmptyMat00.EmptyBlock_BlockEmpty__BlockEmptyMat00")
        (Transformation|SetRelativeScale3D _questionblock "0.080978,0.080978,0.080978"))
      (:then_1
        (CallFunction|Brincar)))))

(event Custom|Movimiento_Moneda
  (Components|MoveComponentTo (Variables|Default|GetCylinder) "0, 0,150.000000" "90.000000, 0,0.000000" true true 0.2 false)
  (Components|MoveComponentTo (Variables|Default|GetCylinder) "0, 0, 0" "90.000000, 0,0.000000" true false 0.2 false))

(event Custom|Cubo_movimiento
  (Components|MoveComponentTo (Variables|Default|GetQuestionBlock) "0, 0,40.000000" "0, 0, 0" true true 0.2 false)
  (Components|MoveComponentTo (Variables|Default|GetQuestionBlock) "0, 0,-50.000000" "0, 0, 0" true false 0.2 false))

(event Custom|brincar
  (Utilities|FlowControl|Sequence
    (:then_0
      (CallFunction|CuboMovimiento))
    (:then_1
      (CallFunction|MovimientoMoneda))))

(event EventBeginPlay)

(event Collision|EventActorBeginOverlap
  (params (OtherActor :type Actor%20Object%20Reference)))

(event EventTick
  (params (DeltaSeconds :type Float%20%28single-precision%29)))

(fn ConstructionScript)