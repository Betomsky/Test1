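; Moving platform Blueprint that shuttles its Cube component back and forth between its relative origin and a Desplazamiento offset.
; From BeginPlay, a self-calling Loop event chains two eased MoveComponentTo moves with a short pause at the far end.
; A second Tick-based method steps the root's world location by an increment, but the setup that initializes its endpoints and enables Validacion is disconnected.
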(event Custom|Loop
  (Components|MoveComponentTo (Variables|Default|GetCube) (Variables|Default|GetDesplazamiento) "0, 0, 0" true true 3.0 false)
  (Utilities|FlowControl|Delay 0.2)
  (Components|MoveComponentTo (Variables|Default|GetCube) "0.000000, 0, 0" "0, 0,0.000000" true true 3.0 false)
  (CallFunction|Loop))

(event EventBeginPlay
  (Components|MoveComponentTo (Variables|Default|GetCube) (Variables|Default|GetDesplazamiento) "0, 0, 0" true true 3.0 false)
  (Utilities|FlowControl|Delay 0.2)
  (Components|MoveComponentTo (Variables|Default|GetCube) "0.000000, 0, 0" "0, 0,0.000000" true true 3.0 false)
  (CallFunction|Loop))

(event EventTick
  (params (DeltaSeconds :type Float%20%28single-precision%29))
  (if (Variables|Default|GetValidacion)
    (if (Math|Vector|Equal(Vector) (Variables|Default|GetOffset) (Variables|Default|GetPosicionDestini) 0.0001)
      (Variables|Default|SetVasHaciaAdelante? false)
      (bind _output_get (Variables|Default|SetOffset (+ (Variables|Default|GetOffset) (Variables|Default|GetNewVar_0)) :!label _label))
      (Transformation|SetWorldLocation (Variables|Default|GetDefaultSceneRoot) _output_get false false)
      (if (Math|Vector|Equal(Vector) (Variables|Default|GetOffset) (Variables|Default|GetPosicionOriginal) 0.0001)
        (Variables|Default|SetVasHaciaAdelante? false))
      (elif (Variables|Default|GetVasHaciaAdelante?)
        (bind _output_get_2 (Variables|Default|SetOffset (+ (Variables|Default|GetOffset) (Variables|Default|GetNewVar_0))))
        (Transformation|SetWorldLocation (Variables|Default|GetDefaultSceneRoot) _output_get_2 false false)
        (else
          (goto _label))))))

(fn ConstructionScript)