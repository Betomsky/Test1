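; Damage-zone actor that repeatedly hurts the SideScrollerCharacter while it stays inside its Box trigger, like a burn.
; Box overlaps set or clear SigueAdentro, and entry fires a DoOnce that passes Daño to EstadoDeSalud on the Instancia_Anahuac game instance.
; After short delays it resets the DoOnce and re-triggers through SigueQuemandose while the character remains inside.
; A Daño threshold check enabling Plane collision is left unconnected.
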(event OnComponentBeginOverlap(Box)
  (params (OverlappedComponent :type Primitive%20Component%20Object%20Reference) (OtherActor :type Actor%20Object%20Reference) (OtherComp :type Primitive%20Component%20Object%20Reference) (OtherBodyIndex :type Integer) (bFromSweep :type Boolean) (SweepResult :type Hit%20Result%20Structure%20%28by%20ref%29))
  (Utilities|Casting|CastToSideScrollerCharacter OtherActor)
  (Variables|Default|SetSigue%20adentro true)
  (Utilities|FlowControl|DoOnce false
    (:Completed
      (bind _asinstancia_anahuac (Utilities|Casting|CastToInstancia_Anahuac (Game|GetGameInstance)))
      (Default|EstadoDeSalud _asinstancia_anahuac (Variables|Default|GetDaño))
      (Utilities|FlowControl|Delay 1.0)
      (CallFunction|DañoTardado)
      (Utilities|FlowControl|Delay 0.2)
      (if (Variables|Default|GetSigue%20adentro)
        (CallFunction|SigueQuemandose)))))

(event OnComponentEndOverlap(Box)
  (params (OverlappedComponent :type Primitive%20Component%20Object%20Reference) (OtherActor :type Actor%20Object%20Reference) (OtherComp :type Primitive%20Component%20Object%20Reference) (OtherBodyIndex :type Integer))
  (Utilities|Casting|CastToSideScrollerCharacter OtherActor)
  (Variables|Default|SetSigue%20adentro false))

(event Custom|Daño%20tardado
  (Utilities|FlowControl|DoOnce false) ; enters at Reset
)

(event Custom|Sigue%20quemandose
  (Utilities|FlowControl|DoOnce false
    (:Completed
      (bind _asinstancia_anahuac (Utilities|Casting|CastToInstancia_Anahuac (Game|GetGameInstance)))
      (Default|EstadoDeSalud _asinstancia_anahuac (Variables|Default|GetDaño))
      (Utilities|FlowControl|Delay 1.0)
      (CallFunction|DañoTardado)
      (Utilities|FlowControl|Delay 0.2)
      (if (Variables|Default|GetSigue%20adentro)
        (CallFunction|SigueQuemandose)))))

(event EventBeginPlay)

(fn ConstructionScript)