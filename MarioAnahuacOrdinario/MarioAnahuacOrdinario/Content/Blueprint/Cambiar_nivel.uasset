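; Level-exit trigger actor that sends the side-scroller character to the next level with a pipe-warp effect.
; The first box overlap by the character, gated by DoOnce, disables player input, plays the Mario pipe sound and sets a flag.
; While that flag is set, Tick pushes the character along negative world Y.
; After a short delay, the level referenced by Nivel2 opens.
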(event OnComponentBeginOverlap(Box)
  (params (OverlappedComponent :type Primitive%20Component%20Object%20Reference) (OtherActor :type Actor%20Object%20Reference) (OtherComp :type Primitive%20Component%20Object%20Reference) (OtherBodyIndex :type Integer) (bFromSweep :type Boolean) (SweepResult :type Hit%20Result%20Structure%20%28by%20ref%29))
  (bind _asside_scroller_character (Utilities|Casting|CastToSideScrollerCharacter OtherActor))
  (Utilities|FlowControl|DoOnce false
    (:Completed
      (Input|DisableInput _asside_scroller_character (Game|GetPlayerController 0))
      (Audio|PlaySound2D "/Game/Sonidos/_Mario__Pipe_Warping_Sound_Effect._Mario__Pipe_Warping_Sound_Effect" 1.0 1.0 0.0 0 0)
      (Variables|Default|SetMueve%20Mario true)
      (Utilities|FlowControl|Delay 3.0)
      (Game|OpenLevel(byObjectReference) "/Game/Niveles/Nivel-2.Nivel-2"))))

(event EventBeginPlay)

(event EventTick
  (params (DeltaSeconds :type Float%20%28single-precision%29))
  (if (Variables|Default|GetMueve%20Mario)
    (Pawn|Input|AddMovementInput (stale OnComponentBeginOverlap(Box) _asside_scroller_character) "0,-1.000000, 0" 1.0 false)))

(fn ConstructionScript)