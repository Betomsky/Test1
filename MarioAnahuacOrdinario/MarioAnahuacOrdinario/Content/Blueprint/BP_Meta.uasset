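; BP_Meta is a goal trigger that ends the level when the side-scroller character overlaps its box.
; On overlap it clears all widgets and calls the Instancia_Anahuac game instance to destroy the character and compute score, coin count, rating and final result.
; It then shows the Resultados widget and plays a victory sound.
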(event OnComponentBeginOverlap(Box)
  (params (OverlappedComponent :type Primitive%20Component%20Object%20Reference) (OtherActor :type Actor%20Object%20Reference) (OtherComp :type Primitive%20Component%20Object%20Reference) (OtherBodyIndex :type Integer) (bFromSweep :type Boolean) (SweepResult :type Hit%20Result%20Structure%20%28by%20ref%29))
  (Utilities|Casting|CastToSideScrollerCharacter OtherActor)
  (bind _asinstancia_anahuac (Utilities|Casting|CastToInstancia_Anahuac (Game|GetGameInstance)))
  (Viewport|RemoveAllWidgets)
  (Default|DestruyeAlPersonaje _asinstancia_anahuac)
  (Default|PuntajeS _asinstancia_anahuac)
  (Default|ConteoDeMoneda _asinstancia_anahuac)
  (Default|Calificación _asinstancia_anahuac)
  (Default|ResultadoF _asinstancia_anahuac)
  (bind _returnvalue (UserInterface|CreateWidget "/Game/Blueprint/Resultados.Resultados_C"))
  (UserInterface|Viewport|AddtoViewport _returnvalue 0)
  (Audio|PlaySound2D "/Game/Sound/Old_victory_sound_roblox.Old_victory_sound_roblox" 1.0 1.0 0.0 0 0))

(event EventBeginPlay)

(event Collision|EventActorBeginOverlap
  (params (OtherActor :type Actor%20Object%20Reference)))

(event EventTick
  (params (DeltaSeconds :type Float%20%28single-precision%29)))

(fn ConstructionScript)