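; Reloj is a countdown clock that costs the player a life when time runs out.
; It seeds the Anahuac game instance with the starting time, then a self-calling Delay loop decrements the counter at a set interval, updating the instance's time score, stored time and formatted time.
; At zero it clears StopLoop, which acts as a keep-running flag, and calls QuitaeVida on the instance if the player is a SideScrollerCharacter.
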(event Custom|Loop
  (if (Variables|Default|Getstop_loop)
    (Utilities|FlowControl|Delay (Variables|Default|GetLapso%20de%20tiempo))
    (bind _output_get (Variables|Default|SetContador%20de%20tiempo (- (Variables|Default|GetContador%20de%20tiempo) 1.0)))
    (bind _asinstancia_anahuac (Utilities|Casting|CastToInstancia_Anahuac (Game|GetGameInstance)))
    (Default|PuntajeDeTiempo _asinstancia_anahuac _output_get)
    (Variables|/Game/Blueprints/Instancia_Anahuac.Instancia_Anahuac_C|SetTiempo _asinstancia_anahuac (Variables|Default|GetContador%20de%20tiempo))
    (Default|FormatearElTiempo _asinstancia_anahuac)
    (if (== _output_get 0.0)
      (Variables|Default|Setstop_loop false)
      (Utilities|Casting|CastToSideScrollerCharacter (Game|GetPlayerCharacter 0))
      (Default|QuitaeVida _asinstancia_anahuac)
      (else
        (CallFunction|Loop)))))

(event EventBeginPlay
  (bind _asinstancia_anahuac (Utilities|Casting|CastToInstancia_Anahuac (Game|GetGameInstance)))
  (Variables|/Game/Blueprints/Instancia_Anahuac.Instancia_Anahuac_C|SetTiempo _asinstancia_anahuac (Variables|Default|GetContador%20de%20tiempo))
  (CallFunction|Loop))

(fn ConstructionScript)