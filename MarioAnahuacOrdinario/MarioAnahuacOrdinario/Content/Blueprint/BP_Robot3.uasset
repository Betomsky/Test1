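; BP_Robot3 is an AI-moved robot enemy that patrols between two target actors and can be destroyed for score.
; Chained AIMoveTo calls start on BeginPlay and re-trigger the Loop event while moves succeed.
; Each Box hit lowers RoboSalud and updates the health text, which Tick turns toward the player along with Cube.
; At zero health it spawns an explosion with sound, destroys itself and passes Score to the Instancia_Anahuac game instance.
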(event OnComponentHit(Box)
  (params (HitComponent :type Primitive%20Component%20Object%20Reference) (OtherActor :type Actor%20Object%20Reference) (OtherComp :type Primitive%20Component%20Object%20Reference) (NormalImpulse :type Vector :default "0, 0, 0") (Hit :type Hit%20Result%20Structure%20%28by%20ref%29))
  (CallFunction|QuitarSalud)
  (Rendering|Components|TextRender|SetText (Variables|Default|GetSalud%20robo) (Utilities|Text|ToText(Integer) (Variables|Default|GetRobo_Salud))))

(event Custom|Loop
  (AI|AIMoveTo self (Transformation|GetActorLocation (Variables|Default|GetTarget_Actor_3)) 0 5.0 false
    (:OnSuccess
      (AI|AIMoveTo self (Transformation|GetActorLocation (Variables|Default|GetTarget_Actor_4)) 0 5.0 false
        (:OnSuccess
          (CallFunction|Loop))))))

(event Custom|Quitar%20Salud
  (bind _returnvalue (Transformation|GetActorLocation))
  (bind _output_get (Variables|Default|SetRobo_Salud (- (Variables|Default|GetRobo_Salud) 20)))
  (if (<= _output_get 0)
    (Effects|SpawnEmitteratLocation "/Game/StarterContent/Particles/P_Explosion.P_Explosion" _returnvalue "0, 0, 0" "2.000000,2.000000,2.000000")
    (Audio|PlaySoundatLocation "/Game/StarterContent/Audio/Explosion_Cue.Explosion_Cue" _returnvalue "0, 0, 0" 1.0 1.0 0.0 0 0 0)
    (Utilities|FlowControl|Delay 0.2)
    (Actor|DestroyActor)
    (bind _asinstancia_anahuac (Utilities|Casting|CastToInstancia_Anahuac (Game|GetGameInstance)))
    (Default|Puntaje _asinstancia_anahuac (Variables|Default|GetScore))))

(event EventBeginPlay
  (AI|AIMoveTo self (Transformation|GetActorLocation (Variables|Default|GetTarget_Actor_3)) 0 5.0 false
    (:OnSuccess
      (AI|AIMoveTo self (Transformation|GetActorLocation (Variables|Default|GetTarget_Actor_4)) 0 5.0 false
        (:OnSuccess
          (CallFunction|Loop))))))

(event EventTick
  (params (DeltaSeconds :type Float%20%28single-precision%29))
  (bind _returnvalue (Game|GetPlayerCharacter 0))
  (bind _salud_robo (Variables|Default|GetSalud%20robo))
  (bind _returnvalue_2 (Transformation|GetActorLocation _returnvalue))
  (bind _returnvalue_3 (Transformation|GetWorldLocation _salud_robo))
  (bind _returnvalue_4 (Math|Rotator|FindLookatRotation _returnvalue_3 _returnvalue_2))
  (Transformation|SetWorldRotation (Variables|Default|GetSalud%20robo) _returnvalue_4 false false)
  (Transformation|SetWorldRotation (Variables|Default|GetCube) _returnvalue_4 false false))

(fn ConstructionScript)