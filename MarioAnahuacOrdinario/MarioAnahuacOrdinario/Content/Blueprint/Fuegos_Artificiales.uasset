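; Fireworks actor that sets off a short timed show of particle bursts with explosion sounds.
; The custom event Activarfuegos activates three particle system components in sequence, each paired with a 2D explosion sound and separated by half-second retriggerable delays.
; BeginPlay, overlap and Tick are unused, so the show only runs when that event is called.
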(event Custom|Activar%20fuegos
  (Components|Activation|Activate (Variables|Default|GetParticleSystem) false)
  (Audio|PlaySound2D "/Game/StarterContent/Audio/Explosion02.Explosion02" 1.0 1.0 0.0 0 0)
  (Utilities|FlowControl|RetriggerableDelay 0.5)
  (Components|Activation|Activate (Variables|Default|GetParticleSystem1) false)
  (Audio|PlaySound2D "/Game/StarterContent/Audio/Explosion01.Explosion01" 1.0 1.0 0.0 0 0)
  (Utilities|FlowControl|RetriggerableDelay 0.5)
  (Components|Activation|Activate (Variables|Default|GetParticleSystem2) false)
  (Audio|PlaySound2D "/Game/StarterContent/Audio/Explosion01.Explosion01" 1.0 1.0 0.0 0 0)
  (Utilities|FlowControl|RetriggerableDelay 0.5))

(event EventBeginPlay)

(event Collision|EventActorBeginOverlap
  (params (OtherActor :type Actor%20Object%20Reference)))

(event EventTick
  (params (DeltaSeconds :type Float%20%28single-precision%29)))

(fn ConstructionScript)