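; Bowser is a boss enemy that periodically fires Bala_de_fuego projectiles and randomly jumps.
; A self-calling Repetir event, started from BeginPlay, loops on a delay and spawns each fireball at the Sphere component's transform.
; Tick gates a random jump behind a delay.
; The first time a SideScrollerCharacter overlaps the Box, it subtracts health through QuitarSalud on the Instancia_Anahuac game instance.
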(event OnComponentBeginOverlap(Box)
  (params (OverlappedComponent :type Primitive%20Component%20Object%20Reference) (OtherActor :type Actor%20Object%20Reference) (OtherComp :type Primitive%20Component%20Object%20Reference) (OtherBodyIndex :type Integer) (bFromSweep :type Boolean) (SweepResult :type Hit%20Result%20Structure%20%28by%20ref%29))
  (Utilities|Casting|CastToSideScrollerCharacter OtherActor)
  (Utilities|FlowControl|DoOnce false
    (:Completed
      (bind _asinstancia_anahuac (Utilities|Casting|CastToInstancia_Anahuac (Game|GetGameInstance)))
      (Default|QuitarSalud _asinstancia_anahuac 0 100))))

(event Custom|Repetir
  (Utilities|FlowControl|Delay 5.5)
  (Game|SpawnActorfromClass "/Game/Blueprint/Bala_de_fuego.Bala_de_fuego_C" (Transformation|GetWorldTransform (Variables|Default|GetSphere)) "Undefined" 0 0)
  (CallFunction|Repetir))

(event EventBeginPlay
  (Utilities|FlowControl|Delay 5.5)
  (Game|SpawnActorfromClass "/Game/Blueprint/Bala_de_fuego.Bala_de_fuego_C" (Transformation|GetWorldTransform (Variables|Default|GetSphere)) "Undefined" 0 0)
  (CallFunction|Repetir))

(event EventTick
  (params (DeltaSeconds :type Float%20%28single-precision%29))
  (Utilities|FlowControl|Delay 2.0)
  (if (Math|Random|RandomBool)
    (Character|Jump)))

(fn ConstructionScript)