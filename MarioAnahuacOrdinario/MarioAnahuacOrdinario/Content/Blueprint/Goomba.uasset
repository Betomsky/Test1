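; Goomba enemy for a side-scroller that walks along the Y axis and can be stomped by the player character.
; While alive and Activar is set, Tick drives movement, and a FlipFlop reverses direction when velocity drops to zero after a short delay.
; A player overlap on the head box removes the damage component, squashes and stops it, plays a death sound, then destroys it and calls the GameInstance's score function.
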(event OnComponentBeginOverlap(Box_Cabeza)
  (params (OverlappedComponent :type Primitive%20Component%20Object%20Reference) (OtherActor :type Actor%20Object%20Reference) (OtherComp :type Primitive%20Component%20Object%20Reference) (OtherBodyIndex :type Integer) (bFromSweep :type Boolean) (SweepResult :type Hit%20Result%20Structure%20%28by%20ref%29))
  (Utilities|Casting|CastToSideScrollerCharacter OtherActor)
  (Utilities|FlowControl|DoOnce false
    (:Completed
      (Components|DestroyComponent (Variables|Default|GetBP_daño))
      (Transformation|SetActorScale3D "1.000000,1.000000,0.355000")
      (Components|Movement|StopMovementImmediately (Variables|Character|GetCharacterMovement))
      (Variables|Default|SetEstoyMuerto? true)
      (Audio|PlaySound2D "/Game/Geometry/GoombaDeath.GoombaDeath" 3.0 0.0 0.2 0 0)
      (Utilities|FlowControl|Delay 0.5)
      (Actor|DestroyActor)
      (bind _asinstancia_anahuac (Utilities|Casting|CastToInstancia_Anahuac (Game|GetGameInstance)))
      (Default|PuntajeDeGoomba _asinstancia_anahuac))))

(event Custom|Cambia%20de%20Direcciones
  (Utilities|FlowControl|FlipFlop
    (:A
      (Variables|Default|SetWorld%20Direction "0,-0.100000, 0"))
    (:B
      (Variables|Default|SetWorld%20Direction "0,0.100000, 0"))))

(event EventTick
  (params (DeltaSeconds :type Float%20%28single-precision%29))
  (if (not (Variables|Default|GetEstoyMuerto?))
    (if (Variables|Default|GetActivar%20)
      (Pawn|Input|AddMovementInput (Variables|Default|GetWorld%20Direction) 1.5 false)
      (Utilities|FlowControl|Delay 0.2)
      (if (== (Math|Vector|VectorLength (Transformation|GetVelocity)) 0.0)
        (CallFunction|CambiaDeDirecciones)))))

(fn ConstructionScript)