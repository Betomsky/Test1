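; Game instance for a Mario-style side-scroller, holding health, lives, coins, score and time.
; Pickup and damage events update these values, with 100 coins granting an extra life.
; GameOver plays the death sequence, then reloads the level, or shows the Fin widget and returns to the main menu at zero lives.
; Coin, score, time and health ratings sum into an A–E grade, and a helper formats the timer.
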(event Custom|Destruye%20al%20personaje)

(event Custom|Agregar_monedas
  (params (Valor_moneda :type Integer) (Conteo%20final%20de%20moneda :type Integer))
  (bind _output_get (Variables|Default|SetConteo%20de%20monedas (+ (Variables|Default|GetConteo%20de%20monedas) Valor_moneda)))
  (if (>= _output_get 100)
    (CallFunction|GanarVidas)
    (Variables|Default|SetConteo%20de%20monedas 0)))

(event Custom|Quitar%20Salud
  (params (Sound :type Sound%20Base%20Object%20Reference) (Valor :type Integer))
  (Variables|Default|SetSalud (- (Variables|Default|GetSalud) Valor))
  (Audio|PlaySound2D Sound 1.0 1.0 0.0 0 0)
  (if (<= (Variables|Default|GetSalud) 0)
    (Variables|Default|SetSalud 0)
    (CallFunction|GameOver)))

(event Custom|Puntaje%20de%20Score
  (if (== (Variables|Default|GetScore) 300)
    (Variables|Default|SetPuntaje_de_score 10)
    (else
      (Variables|Default|SetPuntaje_de_score 5))))

(event Custom|Game%20Over
  (if (== (Variables|Default|GetVidas) 0)
    (Default|CallApagenLaMusica)
    (Audio|PlaySound2D "/Game/Sonidos/MarioMuerte.MarioMuerte" 1.0 1.0 0.0 0 0)
    (CallFunction|DestruyeAlPersonaje)
    (bind _asside_scroller_character (Utilities|Casting|CastToSideScrollerCharacter (Game|GetPlayerCharacter 0)))
    (Default|MarioMuere _asside_scroller_character)
    (Utilities|FlowControl|Delay 5.0)
    (bind _returnvalue (UserInterface|CreateWidget "/Game/Blueprint/Fin.Fin_C"))
    (UserInterface|Viewport|AddtoViewport _returnvalue 0)
    (Audio|PlaySound2D "/Game/Sonidos/GameOverSound.GameOverSound" 1.0 1.0 0.0 0 0)
    (Utilities|FlowControl|Delay 9.0)
    (Game|OpenLevel(byObjectReference) "/Game/Niveles/MenuPrincipal.MenuPrincipal")
    (else
      (Default|CallApagenLaMusica)
      (Audio|PlaySound2D "/Game/Sonidos/MarioMuerte.MarioMuerte" 1.0 1.0 0.0 0 0)
      (CallFunction|DestruyeAlPersonaje)
      (bind _asside_scroller_character_2 (Utilities|Casting|CastToSideScrollerCharacter (Game|GetPlayerCharacter 0)))
      (Default|MarioMuere _asside_scroller_character_2)
      (Utilities|FlowControl|Delay 5.0)
      (bind _returnvalue_2 (Game|GetCurrentLevelName true))
      (Game|OpenLevel(byName) (Utilities|String|StringToName _returnvalue_2)))))

(event Custom|Calificación
  (Variables|Default|SetCalificacion%20F (+ (Variables|Default|GetPuntaje_de_moneda) (Variables|Default|GetCalificacion%20F)))
  (Variables|Default|SetCalificacion%20F (+ (Variables|Default|GetCalificacion%20F) (Variables|Default|GetPuntaje_de_score)))
  (Variables|Default|SetCalificacion%20F (+ (Variables|Default|GetCalificacion%20F) (Math|Float|Truncate (Variables|Default|GetPuntaje%20final%20de%20tiempo))))
  (Variables|Default|SetCalificacion%20F (+ (Variables|Default|GetCalificacion%20F) (Variables|Default|GetPuntaje_de_salud)))
  (if (== (Variables|Default|GetCalificacion%20F) 40)
    (Variables|Default|SetResultado%20F "A")
    (elif (== (Variables|Default|GetCalificacion%20F) 35)
      (Variables|Default|SetResultado%20F "B")
      (elif (== (Variables|Default|GetCalificacion%20F) 30)
        (Variables|Default|SetResultado%20F "C")
        (elif (== (Variables|Default|GetCalificacion%20F) 25)
          (Variables|Default|SetResultado%20F "D")
          (elif (== (Variables|Default|GetCalificacion%20F) 20)
            (Variables|Default|SetResultado%20F "E")))))))

(event Custom|Puntaje_s
  (if (== (Variables|Default|GetSalud) 100)
    (Variables|Default|SetPuntaje_de_salud 10)
    (else
      (Variables|Default|SetPuntaje_de_salud 5))))

(event Custom|Conteo%20de%20moneda
  (if (== (Variables|Default|GetConteo%20final%20de%20moneda) 50)
    (Variables|Default|SetPuntaje_de_moneda 10)
    (else
      (Variables|Default|SetPuntaje_de_moneda 5))))

(event Custom|Puntaje%20final%20de%20moneda
  (params (Puntaje%20de%20moneda :type Integer))
  (Variables|Default|SetConteo%20final%20de%20moneda (+ (Variables|Default|GetConteo%20final%20de%20moneda) Puntaje%20de%20moneda)))

(event Custom|Resultado_F
  (if (== (Variables|Default|GetCalificacion%20F) 40)
    (Variables|Default|SetResultado%20F "A")
    (elif (== (Variables|Default|GetCalificacion%20F) 35)
      (Variables|Default|SetResultado%20F "B")
      (elif (== (Variables|Default|GetCalificacion%20F) 30)
        (Variables|Default|SetResultado%20F "C")
        (elif (== (Variables|Default|GetCalificacion%20F) 25)
          (Variables|Default|SetResultado%20F "D")
          (elif (== (Variables|Default|GetCalificacion%20F) 20)
            (Variables|Default|SetResultado%20F "E")))))))

(event Custom|ReiniciarValores
  (Variables|Default|SetConteo%20de%20monedas 0)
  (Variables|Default|SetScore 0)
  (Variables|Default|SetSalud 100)
  (Variables|Default|SetVidas 3))

(event Custom|Puntaje%20de%20Goomba
  (Variables|Default|SetScore (+ (Variables|Default|GetGoomba%20puntaje) (Variables|Default|GetScore))))

(event Custom|Estado%20de%20salud
  (params (Valor%20de%20salud :type Integer))
  (Variables|Default|SetSalud (Math|Integer|Clamp(Integer) (- (Variables|Default|GetSalud) Valor%20de%20salud) 0 100))
  (Audio|PlaySound2D "/Game/Sound/404108__deathscyp__damage-2.404108__deathscyp__damage-2" 1.0 1.0 0.0 0 0)
  (if (== (Variables|Default|GetSalud) 0)
    (CallFunction|QuitaeVida)))

(event Custom|Quitae%20vida
  (Math|Integer|DecrementInt (Variables|Default|GetVidas)
    (:%20%20
      (Variables|Default|SetSalud 100)
      (CallFunction|GameOver))))

(event Custom|Ganar%20vidas
  (Math|Integer|IncrementInt (Variables|Default|GetVidas)
    (:%20%20
      (Audio|PlaySound2D "/Game/Sound/518306__mrthenoronha__extra-life-8-bit.518306__mrthenoronha__extra-life-8-bit" 1.0 1.0 0.0 0 0))))

(event Custom|Formatear%20el%20tiempo
  (bind _tiempo (Variables|Default|GetTiempo))
  (bind _returnvalue (/ _tiempo 6e+01))
  (bind _returnvalue_2 (Math|Float|Truncate _returnvalue))
  (bind _returnvalue_3 (Math|Float|Fraction _returnvalue))
  (bind _returnvalue_4 (Utilities|String|ToString(Integer) _returnvalue_2))
  (bind _returnvalue_5 (* _returnvalue_3 6e+01))
  (bind _returnvalue_6 (Math|Float|Truncate _returnvalue_5))
  (bind _returnvalue_7 (< _returnvalue_6 10))
  (bind _returnvalue_8 (Utilities|String|ToString(Integer) _returnvalue_6))
  ;[1 1 1] Tiempo
  (if (< _returnvalue_2 0)
    (if _returnvalue_7
      (Variables|Default|SetTiempo%20formateado (Utilities|String|Append "0" _returnvalue_4 ":0" _returnvalue_8))
      (else
        (Variables|Default|SetTiempo%20formateado (Utilities|String|Append "0" _returnvalue_4 ":" _returnvalue_8))))
    (elif _returnvalue_7
      (Variables|Default|SetTiempo%20formateado (Utilities|String|Append _returnvalue_4 ":0" _returnvalue_8))
      (else
        (Variables|Default|SetTiempo%20formateado (Utilities|String|Append _returnvalue_4 ":" (Utilities|String|ToString(Integer) _returnvalue_6)))))))

(event Custom|Puntaje
  (params (Puntos :type Integer))
  (Variables|Default|SetScore (+ Puntos (Variables|Default|GetScore))))

(event Custom|Agregar%20Salud
  (if (< (Variables|Default|GetSalud) 100)
    (Variables|Default|SetSalud (+ (Variables|Default|GetSalud) 20))
    (if (>= (Variables|Default|GetSalud) (Variables|Default|GetSaud%20correcta))
      (Variables|Default|SetSalud (+ 100 (- (Variables|Default|GetSalud) (Variables|Default|GetSalud))))
      (bind _returnvalue (Actor|GetActorOfClass "/Game/Blueprint/Salud.Salud_C"))
      (Actor|DestroyActor _returnvalue)
      (if (== (Variables|Default|GetSalud) 100)
        (Variables|Default|SetPuntaje_de_salud 10)
        (else
          (Variables|Default|SetPuntaje_de_salud 5)))
      (else
        (bind _returnvalue_2 (Actor|GetActorOfClass "/Game/Blueprint/Salud.Salud_C"))
        (Actor|DestroyActor _returnvalue_2)
        (if (== (Variables|Default|GetSalud) 100)
          (Variables|Default|SetPuntaje_de_salud 10)
          (else
            (Variables|Default|SetPuntaje_de_salud 5)))))))

(event Custom|Puntaje%20de%20Tiempo
  (params (Conteo_final_de_tiempo :type Float%20%28single-precision%29))
  (if (>= Conteo_final_de_tiempo 2.5e+02)
    (Variables|Default|SetPuntaje%20final%20de%20tiempo 1e+01)
    (else
      (Variables|Default|SetPuntaje%20final%20de%20tiempo 5.0))))

(event Custom|Asigna%20nivel
  (params (Nivel :type String))
  (Variables|Default|SetNivel Nivel))